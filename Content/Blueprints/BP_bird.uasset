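; BP_bird is the player character for what appears to be a Flappy Bird-style game, moving constantly along +X through movement input on Tick.
; BeginPlay shows the start-screen widget and pauses the game.
; JumpAction unpauses and swaps to the in-game UI when IsPaused is set.
; It also launches the bird upward with a Z-override LaunchCharacter, gated by IsJumping and a short Delay as a cooldown.
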(event EventBeginPlay
  (bind _returnvalue (UserInterface|CreateWidget "/Game/UserInterface/UI_start_game.UI_start_game_C"))
  (UserInterface|Viewport|AddtoViewport _returnvalue 0)
  (Game|SetGamePaused true))

(event Collision|EventActorBeginOverlap
  (params (OtherActor :type Actor%20Object%20Reference)))

(event EventTick
  (params (DeltaSeconds :type Float%20%28single-precision%29))
  (Pawn|Input|AddMovementInput "1.000000, 0, 0" 0.5 false))

(event Input|ActionEvents|InputActionJumpAction
  (params (Key :type Key%20Structure :default "None"))
  (:Pressed
    (if (not (Variables|Default|GetisJumping))
      (Character|LaunchCharacter "0.000000,0.000000,500.000000" false true)
      (Variables|Default|SetisJumping true)
      (Utilities|FlowControl|Delay 0.3)
      (Variables|Default|SetisJumping false))))

(event Input|ActionEvents|InputActionJumpAction
  (params (Key :type Key%20Structure :default "None"))
  (:Pressed
    (if (Variables|Default|GetisPaused)
      (Game|SetGamePaused false)
      (Variables|Default|SetisPaused false)
      (Widget|RemovefromParent (stale EventBeginPlay _returnvalue))
      (bind _returnvalue (UserInterface|CreateWidget "/Game/UserInterface/ul_in_game.ul_in_game_C" 0 self))
      (UserInterface|Viewport|AddtoViewport _returnvalue 0))))

(fn ConstructionScript)