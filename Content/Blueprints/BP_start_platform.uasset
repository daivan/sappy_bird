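; BP_start_platform is a level segment for a Flappy Bird-style game that chains the track, awards score and handles failure.
; When BP_bird enters the FloorSpawner volume, it spawns another BP_start_platform at the Arrow transform, extending the level.
; Leaving ScoreCollision increments the bird's Score.
; Touching the floor or either trunk collision restarts the level through a console command.
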(event OnComponentBeginOverlap(FloorSpawner)
  (params (OverlappedComponent :type Primitive%20Component%20Object%20Reference) (OtherActor :type Actor%20Object%20Reference) (OtherComp :type Primitive%20Component%20Object%20Reference) (OtherBodyIndex :type Integer) (bFromSweep :type Boolean) (SweepResult :type Hit%20Result%20Structure%20%28by%20ref%29))
  (Utilities|Casting|CastToBP_bird OtherActor)
  (Game|SpawnActorfromClass "BP_start_platform_C" (Transformation|GetWorldTransform (Variables|Default|GetArrow)) "Undefined" 0 0))

(event OnComponentBeginOverlap(FloorCollision)
  (params (OverlappedComponent :type Primitive%20Component%20Object%20Reference) (OtherActor :type Actor%20Object%20Reference) (OtherComp :type Primitive%20Component%20Object%20Reference) (OtherBodyIndex :type Integer) (bFromSweep :type Boolean) (SweepResult :type Hit%20Result%20Structure%20%28by%20ref%29))
  (Utilities|Casting|CastToBP_bird OtherActor)
  (Development|ExecuteConsoleCommand "RestartLevel" 0))

(event OnComponentEndOverlap(ScoreCollision)
  (params (OverlappedComponent :type Primitive%20Component%20Object%20Reference) (OtherActor :type Actor%20Object%20Reference) (OtherComp :type Primitive%20Component%20Object%20Reference) (OtherBodyIndex :type Integer))
  (bind _asbp_bird (Utilities|Casting|CastToBP_bird OtherActor))
  (Variables|/Game/Blueprints/BP_bird.BP_bird_C|Setscore _asbp_bird (+ (Variables|/Game/Blueprints/BP_bird.BP_bird_C|Getscore _asbp_bird) 1)))

(event OnComponentBeginOverlap(TopTrunkCollision)
  (params (OverlappedComponent :type Primitive%20Component%20Object%20Reference) (OtherActor :type Actor%20Object%20Reference) (OtherComp :type Primitive%20Component%20Object%20Reference) (OtherBodyIndex :type Integer) (bFromSweep :type Boolean) (SweepResult :type Hit%20Result%20Structure%20%28by%20ref%29))
  (Utilities|Casting|CastToBP_bird OtherActor)
  (Development|ExecuteConsoleCommand "RestartLevel" 0))

(event OnComponentBeginOverlap(BottomTrunkCollision)
  (params (OverlappedComponent :type Primitive%20Component%20Object%20Reference) (OtherActor :type Actor%20Object%20Reference) (OtherComp :type Primitive%20Component%20Object%20Reference) (OtherBodyIndex :type Integer) (bFromSweep :type Boolean) (SweepResult :type Hit%20Result%20Structure%20%28by%20ref%29))
  (Utilities|Casting|CastToBP_bird OtherActor)
  (Development|ExecuteConsoleCommand "RestartLevel" 0))

(event EventBeginPlay)

(event Collision|EventActorBeginOverlap
  (params (OtherActor :type Actor%20Object%20Reference)))

(event EventTick
  (params (DeltaSeconds :type Float%20%28single-precision%29)))

(fn ConstructionScript)